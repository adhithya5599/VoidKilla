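; Void Peek gameplay ability that scans beyond a surface the player looks at and tags nearby objects.
; It traces from the avatar's eyes up to the character's MaxPhase, then offsets the scan center along the hit's surface direction.
; After committing, a sphere overlap sends timed void tags to BPI_VoidTaggable actors.
; A scan gameplay cue is removed after the tag delay, but any non-taggable overlap ends the ability immediately.
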(event `self.K2_ActivateAbility`
  (bind _returnvalue (`self.GetAvatarActorFromActorInfo`))
  (bind _scantagduration (`self.ScanTagDuration`))
  (bind (_outlocation _outrotation) (`Actor.GetActorEyesViewPoint` _returnvalue))
  (bind _asbp_third_person_character (cast `/Game/ThirdPerson/Blueprints/BP_ThirdPersonCharacter` _returnvalue))
  (set `self.MaxRange` (`/Game/ThirdPerson/Blueprints/BP_ThirdPersonCharacter.MaxPhase` _asbp_third_person_character))
  (bind (_out_hit _surface_direction _bhit) (`/Game/ThirdPerson/Blueprints/BFL_VoidPhase.TraceForPhase` self _outlocation (`KismetMathLibrary.GetForwardVector` _outrotation) "TraceTypeQuery3" (`self.MaxRange`) true))
  (if _bhit
    (set `self.ScanCenter` (+ (`.Location` (`GameplayStatics.BreakHitResult` _out_hit)) (* _surface_direction (`self.ScanDepth`))))
    (bind _returnvalue_2 (`self.K2_CommitAbility`))
    (`self.K2_AddGameplayCueWithParams` (struct :`TagName` "GameplayCue.Void.Peek.Scan") (`AbilitySystemBlueprintLibrary.MakeGameplayCueParameters` 0.0 0.0 (struct) (struct) (struct) (struct) (struct) (`self.ScanCenter`)))
    (if _returnvalue_2
      (bind _outactors (`KismetSystemLibrary.SphereOverlapActors` (`self.ScanCenter`) (`self.ScanRadius`) (`self.Object Types`)))
      (for _array_element _outactors
        (if (`KismetSystemLibrary.DoesImplementInterface` _array_element "/Game/ThirdPerson/Blueprints/BPI_VoidTaggable.BPI_VoidTaggable_C")
          (message `/Game/ThirdPerson/Blueprints/BPI_VoidTaggable.ApplyVoidTag` _array_element _scantagduration)
          (`AbilityTask_WaitDelay.WaitDelay` _scantagduration
            (:`OnFinish`
              (`self.K2_RemoveGameplayCue` (struct :`TagName` "GameplayCue.Void.Peek.Scan"))
              (`self.K2_EndAbility`)))
          (else
            (`self.K2_EndAbility`))))
      (else
        (`self.K2_EndAbility`)))
    (else
      (`self.K2_EndAbility`))))

(event `self.K2_OnEndAbility`
  (params (bWasCancelled :type Boolean)))