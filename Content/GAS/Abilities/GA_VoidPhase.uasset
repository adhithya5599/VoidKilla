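; GA_VoidPhase is a gameplay ability that teleports the player through a wall they are looking at.
; It traces from the eyes up to the character's phase range, finds the wall's far face, and caches a floor-snapped exit beyond it before committing.
; A phasing effect then spans timed wind-up, travel and exit stages, which fire gameplay cues and hide the character around the teleport, then restore it.
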(event `self.K2_ActivateAbility`
  (bind _returnvalue (`self.GetAvatarActorFromActorInfo`))
  (bind (_outlocation _outrotation) (`Actor.GetActorEyesViewPoint` _returnvalue))
  (bind _returnvalue_2 (`KismetMathLibrary.GetForwardVector` _outrotation))
  (bind _asbp_third_person_character (cast `/Game/ThirdPerson/Blueprints/BP_ThirdPersonCharacter` _returnvalue))
  (set `self.PlayerCharacterRef` _asbp_third_person_character)
  (set `self.MaxPhaseRange` (`/Game/ThirdPerson/Blueprints/BP_ThirdPersonCharacter.MaxPhase` _asbp_third_person_character))
  (set `self.Direction` _returnvalue_2)
  (bind (_out_hit _surface_direction _bhit) (`/Game/ThirdPerson/Blueprints/BFL_VoidPhase.TraceForPhase` self _outlocation _returnvalue_2 "TraceTypeQuery3" (`self.MaxPhaseRange`) true))
  (if _bhit
    (set `self.CachedEntryPoint` (`.Location` (`GameplayStatics.BreakHitResult` _out_hit)))
    (set `self.CachedDirection` _surface_direction)
    (bind (_exit_face_point _bfound) (`/Game/ThirdPerson/Blueprints/BFL_VoidPhase.FindWallExitPoint` self (`self.CachedEntryPoint`) (`self.CachedDirection`) (`self.MaxWallThickness`)))
    (if _bfound
      (set `self.CachedExitFacePoint` _exit_face_point)
      (bind _final_location (`/Game/ThirdPerson/Blueprints/BFL_VoidPhase.SnapLocationToFloor` self (+ (`self.CachedExitFacePoint`) (* (`/Game/ThirdPerson/Blueprints/BFL_VoidPhase.GetFlattenedDirection` (`self.CachedDirection`)) (`self.ExitClearance`))) 100.0 300.0 "TraceTypeQuery1" (`CapsuleComponent.CapsuleHalfHeight` (`Character.CapsuleComponent` (`self.PlayerCharacterRef`)))))
      (set `self.CachedExitLocation` _final_location)
      (bind _returnvalue_3 (`self.K2_CommitAbility`))
      (if _returnvalue_3
        (bind _returnvalue_4 (`self.BP_ApplyGameplayEffectToOwner` "/Game/GAS/Effects/GE_State_Phasing.GE_State_Phasing_C"))
        (set `self.PhasingEffectHandle` _returnvalue_4)
        (`self.K2_AddGameplayCueWithParams` (struct :`TagName` "GameplayCue.Void.Phase.Windup") (`AbilitySystemBlueprintLibrary.MakeGameplayCueParameters` 0.0 0.0 (struct) (struct) (struct) (struct) (struct) (`self.CachedEntryPoint`) (* (`self.CachedDirection`) -1.0)))
        (`AbilityTask_WaitDelay.WaitDelay` (`self.WindUpDuration`)
          (:`OnFinish`
            (`self.K2_RemoveGameplayCue` (struct :`TagName` "GameplayCue.Void.Phase.Windup"))
            (`self.K2_ExecuteGameplayCueWithParams` (struct :`TagName` "GameplayCue.Void.Phase.Travel") (`AbilitySystemBlueprintLibrary.MakeGameplayCueParameters` 0.0 0.0 (struct) (struct) (struct) (struct) (struct) (`Actor.K2_GetActorLocation` (`self.GetAvatarActorFromActorInfo`))))
            (bind _asbp_third_person_character_2 (cast `/Game/ThirdPerson/Blueprints/BP_ThirdPersonCharacter` (`self.GetAvatarActorFromActorInfo`)))
            (`/Game/ThirdPerson/Blueprints/BP_ThirdPersonCharacter.ChangeMaterialOnVisible` _asbp_third_person_character_2 false)
            (`AbilityTask_WaitDelay.WaitDelay` (`self.TravelStartDuration`)
              (:`OnFinish`
                (`/Game/ThirdPerson/Blueprints/BP_ThirdPersonCharacter.HideCharacterAndCollision` _asbp_third_person_character_2 false)
                (bind _returnvalue_5 (`Actor.K2_TeleportTo` _asbp_third_person_character_2 (`self.CachedExitLocation`) (`KismetMathLibrary.MakeRotFromX` (`self.CachedDirection`))))
                (if _returnvalue_5
                  (`self.K2_ExecuteGameplayCueWithParams` (struct :`TagName` "GameplayCue.Void.Phase.Exit") (`AbilitySystemBlueprintLibrary.MakeGameplayCueParameters` 0.0 0.0 (struct) (struct) (struct) (struct) (struct) (`Actor.K2_GetActorLocation` (`self.GetAvatarActorFromActorInfo`))))
                  (`AbilityTask_WaitDelay.WaitDelay` (`self.TravelStartDuration`)
                    (:`OnFinish`
                      _)))
                (`/Game/ThirdPerson/Blueprints/BP_ThirdPersonCharacter.ChangeMaterialOnVisible` _asbp_third_person_character_2 true)
                (`/Game/ThirdPerson/Blueprints/BP_ThirdPersonCharacter.HideCharacterAndCollision` _asbp_third_person_character_2 true)
                (`self.BP_RemoveGameplayEffectFromOwnerWithHandle` (`self.PhasingEffectHandle`))
                (`self.K2_EndAbility`)))))
        (else
          (`self.K2_EndAbility`)))
      (else
        (`self.K2_EndAbility`)))
    (else
      (`self.K2_EndAbility`))))